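; First-person player character with movement, mouse look, pause menus, debug speed keys, a locker interaction trace and a gravity gun.
; Right mouse traces and grabs light physics objects via a PhysicsHandle that Tick drives to a camera-attached point, while left mouse launches them with effects.
; Tick also outlines faced interface actors through custom depth.
; Voice-over tutorial flags chain through gun use; obsolete crouch, flashlight, ladder and radio-call logic remains disconnected.
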(event `InputAxis|Move For/Back`
  (params (AxisValue :type "Float (single-precision)"))
  ;[1 1 1] Movement(WASD)
  (`self.AddMovementInput` (`self.GetActorForwardVector`) AxisValue))

(event `InputAxis|Move Right/Left`
  (params (AxisValue :type "Float (single-precision)"))
  ;[1 1 1] Movement(WASD)
  (`self.AddMovementInput` (`self.GetActorRightVector`) AxisValue))

(event `Key|Add`
  (params (Key :type "Key Structure" :default "AnyKey"))
  (bind _charactermovement (`self.CharacterMovement`))
  ;[1 1 1] Walk Cheat
  (:`Pressed`
    (set `CharacterMovementComponent.MaxWalkSpeed` (* (`CharacterMovementComponent.MaxWalkSpeed` _charactermovement) 2.0) _charactermovement)))

(event `RaycastToLocker`
  ;[1 1 1] RaycastToLocker
  (bind _outhit (`KismetSystemLibrary.LineTraceSingle` (.location (`SceneComponent.K2_GetComponentToWorld` (`self.Eyes`))) (.location (`SceneComponent.K2_GetComponentToWorld` (`self.Trace`))) "TraceTypeQuery1"))
  (bind (_bblockinghit _binitialoverlap _time _location _impactpoint _normal _impactnormal _physmat _hitactor) (`GameplayStatics.BreakHitResult` _outhit))
  (if (== _hitactor "/Game/Blueprints/BP_Locker.BP_Locker")
    _
    (else
      _))
  (bind _asbp_locker (cast `/Game/Blueprints/BP_Locker` _hitactor))
  (`/Game/Blueprints/BP_Locker.GetE` _asbp_locker))

(event `Key|Subtract`
  (params (Key :type "Key Structure" :default "AnyKey"))
  (bind _charactermovement (`self.CharacterMovement`))
  ;[1 1 1] Walk Cheat
  (:`Pressed`
    (set `CharacterMovementComponent.MaxWalkSpeed` (* (`CharacterMovementComponent.MaxWalkSpeed` _charactermovement) 0.5) _charactermovement)))

(event `Key|Enter`
  (params (Key :type "Key Structure" :default "AnyKey"))
  ;[1 1 1] Walk Cheat
  (:`Pressed`
    (set `CharacterMovementComponent.MaxWalkSpeed` 300.0 (`self.CharacterMovement`))))

(event `BeginnPlay2`
  ;[1 1 1] Obsolete - Radiocall & Call UI
)

(event `BeginPlay3`
  ;[1 1 1] Obsolet - Anfangs Matinee
)

(event `AcceptCall`
  ;[1 1 1] Obsolete - Radiocall & Call UI
)

(event `ExecuteTrigger`
  ;[1 1 1] Obsolete - Radiocall & Call UI
)

(event `EnableMOve`
  (bind _camera (`self.Camera`))
  (bind _transformcomponent (`PlayerCameraManager.TransformComponent` (`GameplayStatics.GetPlayerCameraManager` 0)))
  ;[1 1 1] Obsolet - Anfangs Matinee
  (set `self.CanMove` true)
  (`self.SetActorEnableCollision` true)
  (set `CharacterMovementComponent.GravityScale` 1.0 (`self.CharacterMovement`))
  (`SceneComponent.K2_SetWorldRotation` _camera (`KismetMathLibrary.MakeRotator` 0.0 0.0 (.yaw (`SceneComponent.K2_GetComponentRotation` _camera))) false false)
  (`SceneComponent.K2_SetWorldRotation` _transformcomponent (`KismetMathLibrary.MakeRotator` 0.0 0.0 (.yaw (`SceneComponent.K2_GetComponentRotation` _transformcomponent))) false false))

(event `DisableCallUI`
  ;[1 1 1] Obsolete - Radiocall & Call UI
)

(event `CallUI`
  ;[1 1 1] Obsolete - Radiocall & Call UI
)

(event `InputAxis|Look Up`
  (params (AxisValue :type "Float (single-precision)"))
  ;[1 1 1] Smooth Motion
  (`self.AddControllerPitchInput` AxisValue))

(event `InputAxis|Look Sides`
  (params (AxisValue :type "Float (single-precision)"))
  ;[1 1 1] Smooth Motion
  (`self.AddControllerYawInput` AxisValue))

(event `Repeat`
  ;[1 1 1] Obsolete - Radiocall & Call UI
)

(event `InputAction|Interact`
  (params (Key :type "Key Structure" :default "AnyKey"))
  ;[1 1 1] Action Interact - Cast Functions
  (:`Pressed`
    (`self.RaycastToLocker`)))

(event `ControllCallUI`
  ;[1 1 1] Obsolete - Radiocall & Call UI
)

(event `Key|Escape`
  (params (Key :type "Key Structure" :default "AnyKey"))
  ;[1 1 1] ESC For Menu
  (:`Pressed`
    (`GameplayStatics.SetGamePaused` true)
    (set `PlayerController.bShowMouseCursor` true (`GameplayStatics.GetPlayerController` 0))
    (bind _returnvalue (`|CreateWidget` "/Game/Menü/PauseMenu/Pause.Pause_C"))
    (`UserWidget.AddToViewport` _returnvalue 0)))

(event `InputAction|Flashlight`
  (params (Key :type "Key Structure" :default "AnyKey"))
  ;[1 1 1] Obsolet - Flashlight
)

(event `MakeFlashlightBrighter`
  ;[1 1 1] Obsolet - Flashlight
)

(event `Key|M` :paused true
  (params (Key :type "Key Structure" :default "AnyKey"))
  ;[1 1 1] Alternative Escape Menu for Testing Purposes (By Daniel)
  (:`Pressed`
    (if (`self.IsMenuOpen`)
      (bind _asrestless_game_instance (cast `/Game/Menü/RestlessGameInstance` (`GameplayStatics.GetGameInstance`)))
      (bind _asslider_shit (cast `/Game/Menü/SliderShit` (`/Game/Menü/RestlessGameInstance.MenuWidget` _asrestless_game_instance)))
      (`/Game/Menü/SliderShit.Close_PauseMenu` _asslider_shit)
      (else
        (bind _asrestless_game_instance_2 (cast `/Game/Menü/RestlessGameInstance` (`GameplayStatics.GetGameInstance`)))
        (bind _asslider_shit_2 (cast `/Game/Menü/SliderShit` (`/Game/Menü/RestlessGameInstance.MenuWidget` _asrestless_game_instance_2)))
        (`/Game/Menü/SliderShit.Open_PauseMenu` _asslider_shit_2)))))

(event `Ladder`
  ;[1 1 1] Obsolet - Q - for Ladder
)

(event `InputAxisKey|MouseX`
  (params (AxisValue :type "Float (single-precision)"))
  ;[1 1 1] Look in different directions
  (`SceneComponent.K2_SetWorldRotation` (`self.Camera`) (`self.GetControlRotation`) false false :!label _label))

(event `InputAction|Crouch`
  (params (Key :type "Key Structure" :default "AnyKey"))
  ;[1 1 1] Obsolet - Crouch
)

(event `InputAxisKey|MouseY`
  (params (AxisValue :type "Float (single-precision)"))
  ;[1 1 1] Look in different directions
  (goto _label))

(event `Initialize Moving Speed`
  ;[1 1 1] Obsolet - Crouch
)

(event `self.ReceiveBeginPlay`
  ;[1 1 1] Initialize UI Events / Moving Speed
  (`self.MakeFlashlightBrighter`)
  (`self.BeginPlay3`)
  (`self.BeginnPlay2`)
  (`self.Initialize Moving Speed`))

(event `FUIPressEOn`
  ;[1 1 1] Obsolet - Press E & Call UI
)

(event `FUIPressEOff`
  ;[1 1 1] Obsolet - Press E & Call UI
  (`SceneComponent.SetVisibility` (`self.E`) false false))

(event `FUIFuseOn`
  ;[1 1 1] Obsolet - Press E & Call UI
  (`SceneComponent.SetVisibility` (`self.Fuse`) true false))

(event `FUIFuseOff`
  ;[1 1 1] Obsolet - Press E & Call UI
  (`SceneComponent.SetVisibility` (`self.Fuse`) false false))

(event `UICallOn`
  ;[1 1 1] Obsolet - Press E & Call UI
  (`SceneComponent.SetVisibility` (`self.Call`) true false))

(event `UICallOff`
  ;[1 1 1] Obsolet - Press E & Call UI
  (`SceneComponent.SetVisibility` (`self.Call`) false false))

(event `GetTask`
  ;[1 0 0] GetTask - Event
  (`KismetSystemLibrary.Delay` 1.0)
  (`GameplayStatics.SpawnSoundAttached` "/Game/Sounds/Voice/OffVoice/OffVoice_Beginning_Robert.OffVoice_Beginning_Robert" (`self.Camera`))
  (`KismetSystemLibrary.Delay` 16.3)
  (`GameplayStatics.SpawnSoundAttached` "/Game/Sounds/Voice/OffVoice/OffVoice_RightMouse.OffVoice_RightMouse" (`self.Camera`))
  (`KismetSystemLibrary.Delay` 15.935)
  (set `self.RightMouseSound` true))

(event `Key|C`
  (params (Key :type "Key Structure" :default "AnyKey"))
  ;[1 1 1] Obsolet - Cheat Menu
)

(event `PickUp Object`
  (bind _camera (`self.Camera`))
  (bind _returnvalue (`SceneComponent.K2_GetComponentLocation` _camera))
  ;[1 0 0] PickUp Object Event
  (bind (_outhit _returnvalue_2) (`KismetSystemLibrary.LineTraceSingle` _returnvalue (+ _returnvalue (* (`SceneComponent.GetForwardVector` _camera) (`self.Maximum Pull Distance`))) "TraceTypeQuery1"))
  (if _returnvalue_2
    (bind (_bblockinghit _binitialoverlap _time _location _impactpoint _normal _impactnormal _physmat _hitactor _hitcomponent _hitbonename) (`GameplayStatics.BreakHitResult` _outhit))
    (if (`SceneComponent.IsSimulatingPhysics` _hitcomponent "None")
      (bind _returnvalue_3 (< (`PrimitiveComponent.GetMass` _hitcomponent) (`self.MaximumPullMass`)))
      (if _returnvalue_3
        (`|ExecutionSequence`
          (:`then_0`
            ;[1 1 0] VFX / SFX - Activate Pull
            (`ActorComponent.Activate` (`self.PS_Pull_Mesh`) false)
            (`ActorComponent.Activate` (`self.PS_Pull_Beam`) false)
            (`ParticleSystemComponent.SetBeamTargetPoint` (`self.PS_Pull_Beam`) 0 _location 0)
            (if _returnvalue_3
              ;;[0 0 0] Pull Sound ---> needs to be implemented
              (`GameplayStatics.SpawnSoundAtLocation` "/Game/Sounds/SFX/Christian/Gravity_Gun4_pull_v_2.Gravity_Gun4_pull_v_2" (`SceneComponent.K2_GetComponentLocation` (`self.Camera`)) (struct) 1.4 1.0)))
          (:`then_1`
            (`PhysicsHandleComponent.GrabComponentAtLocationWithRotation` :`self` (`self.PhysicsHandle`) :`Component` _hitcomponent :`InBoneName` _hitbonename :`Location` (`SceneComponent.K2_GetComponentLocation` _hitcomponent))
            (set `self.IsHoldingObject` true)
            (if (`self.RightMouseSound`)
              (`GameplayStatics.SpawnSoundAttached` "/Game/Sounds/Voice/OffVoice/OffVoice_LeftMouse.OffVoice_LeftMouse" (`self.Camera`))
              (`KismetSystemLibrary.Delay` 4.71)
              (set `self.LeftMouseSound` true)
              (set `self.RightMouseSound` false))))))))

(event `Key|RightMouseButton`
  (params (Key :type "Key Structure" :default "AnyKey"))
  ;[0 0 1] Gravity - Input (RightMouseButton; LeftMouseButton)
  (:`Pressed`
    (if (`self.IsHoldingObject`)
      (`self.Drop Object`)
      (else
        (`self.PickUp Object`)))))

(event `Key|LeftMouseButton`
  (params (Key :type "Key Structure" :default "AnyKey"))
  ;[0 0 1] Gravity - Input (RightMouseButton; LeftMouseButton)
  (:`Pressed`
    (if (`self.IsHoldingObject`)
      (`|ExecutionSequence`
        (:`then_0`
          (`self.Launch Object`))
        (:`then_1`
          ;[1 1 0] VFX / SFX - Activate Push; Deactivate Pull
          (`ActorComponent.Activate` (`self.PS_Push`) false)
          ;;[0 0 0] Push Sound ---> needs to be implemented
          (`GameplayStatics.PlaySoundAtLocation` "/Game/Sounds/SFX/Christian/Gravity_Gun4_push_v_2.Gravity_Gun4_push_v_2" (`SceneComponent.K2_GetComponentLocation` (`self.HeldObjectLoacation`)) (struct) 1.4))
        (:`then_2`
          ;[0.23 0.1098 0.04181] Camera Shake - Played at Push / Launch
          (`PlayerCameraManager.PlayCameraShake` :`self` (`GameplayStatics.GetPlayerCameraManager` 0) :`ShakeClass` "/Game/Fabi/BP_Push_CameraShake.BP_Push_CameraShake_C"))))))

(event `Launch Object`
  ;[1 0 0] Launch Object Event
  (if (`self.IsHoldingObject`)
    (`self.Drop Object`)
    (`PrimitiveComponent.AddImpulse` (`.HitComponent` (`GameplayStatics.BreakHitResult` (stale `PickUp Object` _outhit))) (* (`SceneComponent.GetForwardVector` (`self.Camera`)) (`self.Push Impulse Amount`)) "None" true)
    (if (`self.LeftMouseSound`)
      (set `self.LeftMouseSound` false)
      (`GameplayStatics.SpawnSoundAttached` "/Game/Sounds/Voice/OffVoice/OffVoice_ShootTease.OffVoice_ShootTease" (`self.Camera`))
      (`KismetSystemLibrary.Delay` 15.35)
      (`AddComponent|NODE_AddAudioComponent-2`))))

(event `Drop Object`
  ;[1 0 0] Drop Object Event
  (`ActorComponent.Deactivate` (`self.PS_Pull_Beam`))
  (`ActorComponent.Deactivate` (`self.PS_Pull_Mesh`))
  (`PhysicsHandleComponent.ReleaseComponent` (`self.PhysicsHandle`))
  (set `self.IsHoldingObject` false))

(event `self.ReceiveTick`
  (params (DeltaSeconds :type "Float (single-precision)"))
  (bind _returnvalue (`SceneComponent.K2_GetComponentLocation` (`self.HeldObjectLoacation`)))
  (bind _location (.location (`SceneComponent.K2_GetComponentToWorld` (`self.Camera`))))
  ;[1 0 0] Event Tick - Update Objects Position and Rotation by SceneComponent (Parent of SceneComponent is Camera)
  (`|ExecutionSequence`
    (:`then_0`
      (`PhysicsHandleComponent.SetTargetLocation` (`self.PhysicsHandle`) _returnvalue)
      (`PhysicsHandleComponent.SetTargetRotation` (`self.PhysicsHandle`) (`SceneComponent.K2_GetComponentRotation` (`self.HeldObjectLoacation`)))
      (`ParticleSystemComponent.SetBeamTargetPoint` (`self.PS_Pull_Beam`) 0 _returnvalue 0))
    (:`then_1`
      ;[1 0.4028 0] Used to define Outlines at Objects, the Player is facing
      (bind (_outhit _returnvalue_2) (`KismetSystemLibrary.LineTraceSingle` _location (+ _location (* (`KismetMathLibrary.GetForwardVector` (.rotation (`SceneComponent.K2_GetComponentToWorld` (`self.Camera`)))) (`self.Maximum Pull Distance`))) "TraceTypeQuery1"))
      (if _returnvalue_2
        (bind (_bblockinghit _binitialoverlap _time _location_2 _impactpoint _normal _impactnormal _physmat _hitactor) (`GameplayStatics.BreakHitResult` _outhit))
        (if (`KismetSystemLibrary.DoesImplementInterface` _hitactor "/Game/Blueprints/BP_OutlinedObjects.BP_OutlinedObjects_C")
          (message `/Game/Blueprints/BP_OutlinedObjects.NewFunction_0` _hitactor)
          (`/Engine/EditorBlueprintResources/StandardMacros.IsValid` (`self.LastFacedObject`)
            (:`Is Valid`
              (if (== (`self.CurrentFacedObject`) (`self.LastFacedObject`))
                (`PrimitiveComponent.SetRenderCustomDepth` (`self.CurrentFacedObject`) true)
                (else
                  (`PrimitiveComponent.SetRenderCustomDepth` (`self.CurrentFacedObject`) true)
                  (`PrimitiveComponent.SetRenderCustomDepth` (`self.LastFacedObject`) false)
                  (set `self.LastFacedObject` (`self.CurrentFacedObject`)))))
            (:`Is Not Valid`
              (set `self.LastFacedObject` (`self.CurrentFacedObject`))))
          (else
            (`/Engine/EditorBlueprintResources/StandardMacros.IsValid` (`self.LastFacedObject`)
              (:`Is Valid`
                (`PrimitiveComponent.SetRenderCustomDepth` (`self.LastFacedObject`) false)))))
        (else
          ;;[1 1 1] Deactivate CustomRenderDepth while getting invalid input
          (`/Engine/EditorBlueprintResources/StandardMacros.IsValid` (`self.CurrentFacedObject`)
            (:`Is Valid`
              (`PrimitiveComponent.SetRenderCustomDepth` (`self.CurrentFacedObject`) false)
              (set `self.CurrentFacedObject` null))))))))

(fn `UserConstructionScript`)