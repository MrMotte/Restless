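; BP_Locker is a locker with a door that toggles between two positions.
; At BeginPlay it binds SwitchDoor through BindEventToGetE, and each call flip-flops a timeline forward or in reverse.
; The timeline drives a rotator lerp on the Arrow component's relative rotation, swinging it through 90 degrees.
; A Box component tracks overlap in an Overlapping flag, which the door toggle does not check here.
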(event `self.ReceiveBeginPlay`
  (add `self.GetE` (delegate `SwitchDoor`)))

(event `SwitchDoor`
  (`/Engine/EditorBlueprintResources/StandardMacros.FlipFlop`
    (:`A`
      (bind (_direction _newtrack_0) (`Timeline|Timeline_0` :!label _label)
        (:`Update`
          (`SceneComponent.K2_SetRelativeRotation` (`self.Arrow`) (`KismetMathLibrary.RLerp` (struct :`Yaw` 90.0) (struct) _newtrack_0) false false))))
    (:`B`
      (goto _label :!via `Reverse`))))

(event `self.Box.OnComponentBeginOverlap`
  (params (OverlappedComponent :type "PrimitiveComponent Object Reference") (OtherActor :type "Actor Object Reference") (OtherComp :type "PrimitiveComponent Object Reference") (OtherBodyIndex :type Integer) (bFromSweep :type Boolean) (SweepResult :type "HitResult Structure (by ref)"))
  (set `self.Overlapping?` true))

(event `self.Box.OnComponentEndOverlap`
  (params (OverlappedComponent :type "PrimitiveComponent Object Reference") (OtherActor :type "Actor Object Reference") (OtherComp :type "PrimitiveComponent Object Reference") (OtherBodyIndex :type Integer))
  (set `self.Overlapping?` false))

(fn `UserConstructionScript`)