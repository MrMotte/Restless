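; BP_Pointlight is a point light actor meant to react to reactor power, with most of that logic now obsolete and disconnected.
; EnableEnergy still plays a timeline that ramps intensity between 1% and 100% of DefaultIntensity, but its binding to BP_Reactor never runs.
; The orphaned break logic played a reversed flicker timeline and broken-door sound, then cleared the reactor's EnergyState once.
; BeginPlay is empty, so DefaultIntensity is never captured here.
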(event `self.ReceiveBeginPlay`
  ;[1 1 1] Obsolet - Disable Light on Energy Broken
)

(event `OnEnergyBrokeTriggerOverlap`
  ;[1 1 1] Obsolet - Disable Light on Energy Broken
)

(event `GetEnableEnergy`
  ;[1 1 1] Obsolet - Enable Light on Interact with Reactor
)

(event `Enable Energy`
  (bind _defaultintensity (`self.DefaultIntensity`))
  ;[1 1 1] Obsolet - Enable Light on Interact with Reactor
  (bind (_direction _newtrack_1) (`Timeline|Timeline_0` :!via `PlayFromStart`)
    (:`Update`
      (`LightComponent.SetIntensity` (`self.PointLight`) (`KismetMathLibrary.Lerp` (* _defaultintensity 0.01) _defaultintensity _newtrack_1)))))

(fn `UserConstructionScript`)