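; BP_Reactor is an interactable reactor that the player switches on once to enable energy.
; A Box overlap toggles the character's press-E prompt and gates the Interact event.
; On first activation it calls CallEnableEnergy, permanently disables the prompt and plays a start sound at a hardcoded location.
; A timeline then drives the spotlight color and the volume of the hum and water pipe audio.
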(event `Interact`
  (if (`PrimitiveComponent.IsOverlappingActor` (`self.Box`) (`GameplayStatics.GetPlayerCharacter` 0))
    (if (not (`self.EnergyState`))
      (`self.EnableEnergy`)
      (set `self.EnergyState` true)
      (set `self.DisableUI` true)
      (`self.Disable`)
      (`GameplayStatics.PlaySoundAtLocation` "/Game/Sounds/SFX/ReactorStartCue.ReactorStartCue" (565.0 11.0 841.0))
      (bind (_direction _newtrack_0 _newtrack_2) (`Timeline|Timeline_0` :!via `PlayFromStart`)
        (:`Update`
          (`LightComponent.SetLightColor` (`self.SpotLight`) _newtrack_2 true)
          (`AudioComponent.SetVolumeMultiplier` (`self.ReactorHumCue`) _newtrack_0)
          (`AudioComponent.SetVolumeMultiplier` (`self.WaterPipeLeft`) _newtrack_0)
          (`AudioComponent.SetVolumeMultiplier` (`self.WaterPipeRight`) _newtrack_0))))))

(event `self.Box.OnComponentBeginOverlap`
  (params (OverlappedComponent :type "PrimitiveComponent Object Reference") (OtherActor :type "Actor Object Reference") (OtherComp :type "PrimitiveComponent Object Reference") (OtherBodyIndex :type Integer) (bFromSweep :type Boolean) (SweepResult :type "HitResult Structure (by ref)"))
  (if (not (`self.DisableUI`))
    (bind _asbp_character_player (cast `/Game/Fabi/BP_Character_Player` (`GameplayStatics.GetPlayerCharacter` 0)))
    (`/Game/Fabi/BP_Character_Player.LBUIPressEOn` _asbp_character_player)))

(event `Disable`
  (bind _asbp_character_player (cast `/Game/Fabi/BP_Character_Player` (`GameplayStatics.GetPlayerCharacter` 0) :!label _label))
  (`/Game/Fabi/BP_Character_Player.LBUIPressEOff` _asbp_character_player))

(event `self.Box.OnComponentEndOverlap`
  (params (OverlappedComponent :type "PrimitiveComponent Object Reference") (OtherActor :type "Actor Object Reference") (OtherComp :type "PrimitiveComponent Object Reference") (OtherBodyIndex :type Integer))
  (goto _label))

(fn `UserConstructionScript`)