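; BP_CryoPod is a cryo pod actor that animates its chamber door and rotates a Box component when play begins.
; The Door event casts the first actor tagged MyLittleCryo to BP_CryoPod, waits briefly, then uses a timeline to lerp that pod's door roll in world space, rather than targeting itself directly.
; A second timeline's event track adds local yaw steps to the Box.
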(event `Door`
  (bind _outactors (`GameplayStatics.GetAllActorsWithTag` "MyLittleCryo"))
  (bind _asbp_cryo_pod (cast `/Game/Blueprints/BP_CryoPod` (`KismetArrayLibrary.Array_Get` _outactors)))
  (`KismetSystemLibrary.Delay` 5.0)
  (bind (_direction _newtrack_9) (`Timeline|Timeline_1`)
    (:`Update`
      (`SceneComponent.K2_SetWorldRotation` (`/Game/Blueprints/BP_CryoPod.CryoChamberDoor` _asbp_cryo_pod) (`KismetMathLibrary.MakeRotator` (`KismetMathLibrary.Lerp` -90.0 0.0 _newtrack_9) 0.0 45.0) false false))))

(event `self.ReceiveBeginPlay`
  (`self.Door`)
  (`Timeline|Timeline_0`
    (:`NewTrack_8`
      (`SceneComponent.K2_AddLocalRotation` (`self.Box`) (`KismetMathLibrary.MakeRotator` 0.0 0.0 1.0) false false))))

(fn `UserConstructionScript`)