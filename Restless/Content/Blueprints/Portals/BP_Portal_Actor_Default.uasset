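; Default portal actor that shows a live view through to a target portal and teleports actors overlapping its trigger.
; A scene capture, fed into a dynamic material on the portal plane, follows the player camera relative to both portals each tick, with a clip plane at the target.
; The target transform can be rotated 180 degrees, the render texture follows viewport resizes, and a temporary ignore list stops arriving actors re-triggering teleport.
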(event `self.ReceiveBeginPlay`
  (`parent.ReceiveBeginPlay`)
  (`|ExecutionSequence`
    (:`then_0`
      (bind _returnvalue (`KismetMaterialLibrary.CreateDynamicMaterialInstance` "/PortalPlugin/Materials/M_FlatPortal_Master.M_FlatPortal_Master"))
      (bind _output_get (set `self.Portal MID Center` _returnvalue))
      (`PrimitiveComponent.SetMaterial` (`self.Portal Plane`) 0 _output_get))
    (:`then_1`
      (bind _capture_component (`self.Add Capture Component` (`WidgetLayoutLibrary.GetViewportSize`) (`self.Portal MID Center`)))
      (set `self.Center Capture Component` _capture_component))))

(event `self.ReceiveTick`
  (params (DeltaSeconds :type "Float (single-precision)"))
  (bind _returnvalue (`GameplayStatics.GetPlayerCameraManager` 0))
  (bind _center_capture_component (`self.Center Capture Component`))
  (`parent.ReceiveTick` DeltaSeconds)
  (`PortalFunctionLibrary.UpdateCaptureComponentClipPlaneTransform` _center_capture_component (`self.Get Target Plane Transform`))
  (`PortalFunctionLibrary.UpdateCaptureComponentWithTransforms` _center_capture_component (`KismetMathLibrary.MakeTransform` (`PlayerCameraManager.GetCameraLocation` _returnvalue) (`PlayerCameraManager.GetCameraRotation` _returnvalue)) (`self.Get Source Portal Transform`) (`self.Get Target Portal Transform`)))

(event `self.On Viewport Resized`
  (`self.Update Render Texture` (`WidgetLayoutLibrary.GetViewportSize`) (`self.Center Capture Component`) (`self.Portal MID Center`)))

(event `self.Notify Pre Teleport`
  (params (`Incoming Actor` :type "Actor Object Reference"))
  (`KismetArrayLibrary.Array_Add` (`self.Temporary Ignore List`) `Incoming Actor`))

(event `self.Teleport Trigger.OnComponentBeginOverlap`
  (params (OverlappedComponent :type "PrimitiveComponent Object Reference") (OtherActor :type "Actor Object Reference") (OtherComp :type "PrimitiveComponent Object Reference") (OtherBodyIndex :type Integer) (bFromSweep :type Boolean) (SweepResult :type "HitResult Structure (by ref)"))
  (if (not (`KismetArrayLibrary.Array_Contains` (`self.Temporary Ignore List`) OtherActor))
    (message `/PortalPlugin/Blueprints/BPI_PortalUsingActor.Entered Portal` OtherActor)
    (`self.Teleport Actor` OtherActor)))

(event `self.Teleport Trigger.OnComponentEndOverlap`
  (params (OverlappedComponent :type "PrimitiveComponent Object Reference") (OtherActor :type "Actor Object Reference") (OtherComp :type "PrimitiveComponent Object Reference") (OtherBodyIndex :type Integer))
  (`KismetArrayLibrary.Array_RemoveItem` (`self.Temporary Ignore List`) OtherActor)
  (message `/PortalPlugin/Blueprints/BPI_PortalUsingActor.Exited Portal` OtherActor))

(fn `Get Target Plane Transform`
  (returns (Transform :type "Transform Structure"))
  (bind _target_portal_actor (`self.Target Portal Actor`))
  (bind _asbp_portal_actor_default (cast `/Game/Blueprints/Portals/BP_Portal_Actor_Default` _target_portal_actor)
    (:`then`
      (return (`SceneComponent.K2_GetComponentToWorld` (`/Game/Blueprints/Portals/BP_Portal_Actor_Default.Portal Plane` _asbp_portal_actor_default))))
    (:`CastFailed`
      (return (`self.GetTransform` _target_portal_actor)))))

(fn `Get Target Portal Transform`
  (returns (`Target Transform` :type "Transform Structure"))
  (bind (_transform_location _transform_rotation) (`KismetMathLibrary.BreakTransform` (`self.Get Target Plane Transform`)))
  (return (`KismetMathLibrary.MakeTransform` _transform_location (select `bool` (`self.Rotate Out 180 Degrees`) :`false` _transform_rotation :`true` (`KismetMathLibrary.ComposeRotators` (struct :`Yaw` 180.0) _transform_rotation)))))

(fn `UserConstructionScript`
  (`parent.UserConstructionScript`))