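; Trash chute puzzle actor that counts down barrels dropped into it and opens doors when none remain.
; KillZone destroys overlapping actors, updating the counter text for "Barrel"-tagged ones and playing right or wrong feedback sounds.
; At zero it shows finished text, sets the state of tagged Door2Hell actors and messages the Blockout_beat2 streaming level through an interface.
; Outlined-interface objects hitting the shaft outside Schacht trigger a hurt sound.
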(event `self.ReceiveBeginPlay`
  ;[1 1 1] Initialize Text
  (`TextRenderComponent.K2_SetText` (`self.Count`) (`KismetTextLibrary.Conv_StringToText` (`KismetStringLibrary.Concat_StrStr` "Left" (`KismetTextLibrary.Conv_TextToString` (`KismetTextLibrary.Conv_IntToText` (`self.Counter`)))))))

(event `self.KillZone.OnComponentBeginOverlap`
  (params (OverlappedComponent :type "PrimitiveComponent Object Reference") (OtherActor :type "Actor Object Reference") (OtherComp :type "PrimitiveComponent Object Reference") (OtherBodyIndex :type Integer) (bFromSweep :type Boolean) (SweepResult :type "HitResult Structure (by ref)"))
  (bind _counter (`self.Counter`))
  ;[1 1 1] Compare Tags
  (if (`self.ActorHasTag` OtherActor "Barrel")
    ;[1 1 1] Update Counter, Destroy Actor
    (set `self.Counter` (- _counter 1))
    (`self.K2_DestroyActor` OtherActor)
    (`|ExecutionSequence`
      (:`then_0`
        ;[0 0.07764 1] Play Yummi Sound
        (`ActorComponent.Activate` (`self.RightObject`) false)
        (`KismetSystemLibrary.Delay` 1.0)
        (`ActorComponent.Deactivate` (`self.RightObject`)))
      (:`then_1`
        (if (== _counter 0)
          ;[1 1 1] Update to finished Text and open Door
          (`TextRenderComponent.K2_SetText` (`self.Count`) (`self.TextFinished`))
          (bind _outactors (`GameplayStatics.GetAllActorsWithTag` (`self.DoorTag`)))
          (for _array_element _outactors
            (bind _asdoor_2hell (cast `/Game/modules/Door/Door2Hell` _array_element))
            (set `/Game/modules/Door/Door2Hell.DoorState` "NewEnumerator0" _asdoor_2hell)
            (message `/Game/Blueprints/TheTrashyInterface.TheTrashyInterface` (`GameplayStatics.GetStreamingLevel` "Blockout_beat2")))
          (else
            ;[1 1 1] Update Left Text
            (`TextRenderComponent.K2_SetText` (`self.Count`) (`KismetTextLibrary.Conv_StringToText` (`KismetStringLibrary.Concat_StrStr` "Left " (`KismetTextLibrary.Conv_TextToString` (`KismetTextLibrary.Conv_IntToText` (`self.Counter`))))))))))
    (else
      (`self.K2_DestroyActor` OtherActor)
      ;[0.01923 0.02986 1] Play Bääähhh Sound
      (`ActorComponent.Activate` (`self.FalseObject`) false)
      (`KismetSystemLibrary.Delay` 2.0)
      (`ActorComponent.Deactivate` (`self.FalseObject`)))))

(event `self.GarbageShaft.OnComponentHit`
  (params (HitComponent :type "PrimitiveComponent Object Reference") (OtherActor :type "Actor Object Reference") (OtherComp :type "PrimitiveComponent Object Reference") (NormalImpulse :type "Vector Structure") (Hit :type "HitResult Structure (by ref)"))
  ;[1 1 1] Hitted Trash outside
  (if (`KismetSystemLibrary.DoesImplementInterface` OtherActor "/Game/Blueprints/BP_OutlinedObjects.BP_OutlinedObjects_C")
    (if (not (`PrimitiveComponent.IsOverlappingActor` (`self.Schacht`) OtherActor))
      ;[0.09969 0.04501 1] Play Ouch Sound
      (`ActorComponent.Activate` (`self.HurtSound`) false)
      (`KismetSystemLibrary.Delay` 3.0)
      (`ActorComponent.Deactivate` (`self.HurtSound`)))))

(fn `UserConstructionScript`)