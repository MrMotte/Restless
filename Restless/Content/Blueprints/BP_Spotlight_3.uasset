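; Spotlight actor with leftover logic for dimming and restoring its Spot intensity as energy breaks or returns.
; EnableEnergy plays a timeline that lerps intensity from 1% of DefaultIntensity up to full.
; The BP_Reactor and BP_Pointlight bindings, DefaultIntensity capture and reverse-timeline dimming are disconnected, with the energy graphs marked obsolete.
; BeginPlay and the overlap handler are empty, so nothing here triggers either fade.
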(event `self.ReceiveBeginPlay`
  ;[1 1 1] Obsolet - Disable Light on Energy Broken
)

(event `OnEnergyBrokeTriggerOverlap`
  ;[1 1 1] Obsolet - Disable Light on Energy Broken
)

(event `GetEnableEnergy`
  ;[1 1 1] Obsolet - Enable Energy on Reactor Interact
)

(event `EnableEnergy`
  (bind _defaultintensity (`self.DefaultIntensity`))
  ;[1 1 1] Obsolet - Enable Energy on Reactor Interact
  (bind (_direction _newtrack_1) (`Timeline|Timeline_1` :!via `PlayFromStart`)
    (:`Update`
      (`LightComponent.SetIntensity` (`self.Spot`) (`KismetMathLibrary.Lerp` (* _defaultintensity 0.01) _defaultintensity _newtrack_1)))))

(fn `UserConstructionScript`)