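; Key card pickup that the player collects by interacting while inside its collision volume.
; Actor overlaps toggle custom depth on the mesh, and collision overlaps toggle the player's "Press E" prompt unless collection has disabled it.
; Interact, bound to an AccessCard event dispatcher on BeginPlay, checks player overlap, then hides the mesh, flags the card as collected and clears the prompt.
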(event `self.ReceiveActorBeginOverlap`
  (params (OtherActor :type "Actor Object Reference"))
  (`PrimitiveComponent.SetRenderCustomDepth` (`self.StaticMeshComponent`) true))

(event `self.ReceiveBeginPlay`
  (add `self.AccessCardED` (delegate `Interact`)))

(event `Interact`
  (if (`PrimitiveComponent.IsOverlappingActor` (`self.Collision`) (`GameplayStatics.GetPlayerCharacter` 0))
    (if (not (`self.CollectedAccessCard?`))
      (`SceneComponent.ToggleVisibility` (`self.StaticMeshComponent`) false)
      (set `self.CollectedAccessCard?` true)
      (set `self.DisableUI` true)
      (`self.Disable`))))

(event `self.ReceiveActorEndOverlap`
  (params (OtherActor :type "Actor Object Reference"))
  (`PrimitiveComponent.SetRenderCustomDepth` (`self.StaticMeshComponent`) false))

(event `self.Collision.OnComponentBeginOverlap`
  (params (OverlappedComponent :type "PrimitiveComponent Object Reference") (OtherActor :type "Actor Object Reference") (OtherComp :type "PrimitiveComponent Object Reference") (OtherBodyIndex :type Integer) (bFromSweep :type Boolean) (SweepResult :type "HitResult Structure (by ref)"))
  (if (not (`self.DisableUI`))
    (bind _asbp_character_player (cast `/Game/Fabi/BP_Character_Player` (`GameplayStatics.GetPlayerCharacter` 0)))
    (`/Game/Fabi/BP_Character_Player.LBUIPressEOn` _asbp_character_player)))

(event `self.Collision.OnComponentEndOverlap`
  (params (OverlappedComponent :type "PrimitiveComponent Object Reference") (OtherActor :type "Actor Object Reference") (OtherComp :type "PrimitiveComponent Object Reference") (OtherBodyIndex :type Integer))
  (bind _asbp_character_player (cast `/Game/Fabi/BP_Character_Player` (`GameplayStatics.GetPlayerCharacter` 0) :!label _label))
  (`/Game/Fabi/BP_Character_Player.LBUIPressEOff` _asbp_character_player))

(event `Disable`
  (goto _label))

(fn `UserConstructionScript`)