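; Fuse box where the player, standing in its trigger box with a collected BP_Fuse, can insert the fuse once.
; Interacting hides the press-E prompt, moves the fuse mesh to a hardcoded position, plays a sound and runs a timeline on spotlight color and audio volume.
; BP_Reactor and BP_Pointlight dispatchers drive timelines that fade the spotlight between dimmed and default intensity when energy is enabled or breaks.
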(event `self.ReceiveBeginPlay`
  ;[1 1 1] Put Fuse in Fusebox
  ;;[1 1 1] Steh ich im Trigger?
  (`self.BeginPlay2`)
  (add `self.FuseBoxED` (delegate `Interact`)))

(event `Interact`
  ;[1 1 1] Put Fuse in Fusebox
  ;;[1 1 1] Steh ich im Trigger?
  (if (`PrimitiveComponent.IsOverlappingActor` (`self.Box`) (`GameplayStatics.GetPlayerCharacter` 0))
    ;;[1 1 1] Hab ich die Fuse & hatte ich die Fusebox schon benutzt?
    (bind _outactors (`GameplayStatics.GetAllActorsOfClass` "/Game/Blueprints/BP_Fuse.BP_Fuse_C"))
    (for _array_element _outactors
      (if (`/Game/Blueprints/BP_Fuse.CollectedFuse?` _array_element)
        (if (not (`self.FuseboxAlreadyUsed?`))
          (set `self.FuseboxAlreadyUsed?` true)
          ;;[1 1 1] Schalte UI an
          (bind _outactors_2 (`GameplayStatics.GetAllActorsOfClass` "/Game/Blueprints/BP_Fuse.BP_Fuse_C"))
          (set `/Game/Blueprints/BP_Fuse.FuseUITrigger` false (`KismetArrayLibrary.Array_Get` _outactors_2))
          (set `self.DisableUI` true)
          (`self.Disable`)
          ;;[1 1 1] Setze Fuse in Box ein
          (bind _outactors_3 (`GameplayStatics.GetAllActorsOfClass` "/Game/Blueprints/BP_Fuse.BP_Fuse_C"))
          (for _array_element_2 _outactors_3
            (bind _staticmeshcomponent (`StaticMeshActor.StaticMeshComponent` _array_element_2))
            (`SceneComponent.ToggleVisibility` _staticmeshcomponent false)
            (`SceneComponent.K2_SetRelativeLocationAndRotation` _staticmeshcomponent (-793.0 502.0 156.0) (struct :`Yaw` -45.0) false true)
            ;;[1 1 1] Spiele Sound und ändere Spotlight farbe
            (`GameplayStatics.PlaySoundAtLocation` "/Game/Sounds/SFX/PlaceFuseCue.PlaceFuseCue" (-793.0 501.0 156.0))
            (bind (_direction _newtrack_1 _newtrack_2) (`Timeline|Timeline_0` :!via `PlayFromStart`)
              (:`Update`
                (`LightComponent.SetLightColor` (`self.SpotLight`) _newtrack_2 true)
                (`AudioComponent.SetVolumeMultiplier` (`self.Audio`) _newtrack_1)))))))))

(event `BeginPlay2`
  ;[1 1 1] Put Fuse in Fusebox
  (`self.GetEnableEnergy`)
  (set `self.DefaultIntensity` (`LightComponentBase.Intensity` (`self.SpotLight`)))
  (bind _outactors (`GameplayStatics.GetAllActorsOfClass` "/Game/Blueprints/BP_Pointlight.BP_Pointlight_C"))
  (add `/Game/Blueprints/BP_Pointlight.GetEnergyBrokeTriggerOverlapp` (`KismetArrayLibrary.Array_Get` _outactors) (delegate `EnergyBroke`)))

(event `self.Box.OnComponentBeginOverlap`
  (params (OverlappedComponent :type "PrimitiveComponent Object Reference") (OtherActor :type "Actor Object Reference") (OtherComp :type "PrimitiveComponent Object Reference") (OtherBodyIndex :type Integer) (bFromSweep :type Boolean) (SweepResult :type "HitResult Structure (by ref)"))
  ;[1 1 1] Put Fuse in Fusebox
  ;;[1 1 1] Enable/Disable UI
  (if (not (`self.DisableUI`))
    (bind _asbp_character_player (cast `/Game/Fabi/BP_Character_Player` (`GameplayStatics.GetPlayerCharacter` 0)))
    (`/Game/Fabi/BP_Character_Player.LBUIPressEOn` _asbp_character_player)))

(event `EnergyBroke`
  (bind _defaultintensity (`self.DefaultIntensity`))
  ;[1 1 1] Put Fuse in Fusebox
  (if (not (`/Game/Blueprints/BP_Pointlight.EnergyFirstBroke` (`KismetArrayLibrary.Array_Get` (stale `BeginPlay2` _outactors))))
    (bind _outactors (`GameplayStatics.GetAllActorsOfClass` "/Game/Blueprints/BP_Reactor.BP_Reactor_C"))
    (if (`/Game/Blueprints/BP_Reactor.EnergyState` (`KismetArrayLibrary.Array_Get` _outactors))
      (bind (_direction _newtrack_1) (`Timeline|Timeline_1` :!via `ReverseFromEnd`)
        (:`Update`
          (`LightComponent.SetIntensity` (`self.SpotLight`) (`KismetMathLibrary.Lerp` (* _defaultintensity 0.1) _defaultintensity _newtrack_1)))))))

(event `Disable`
  ;[1 1 1] Put Fuse in Fusebox
  ;;[1 1 1] Enable/Disable UI
  (bind _asbp_character_player (cast `/Game/Fabi/BP_Character_Player` (`GameplayStatics.GetPlayerCharacter` 0) :!label _label))
  (`/Game/Fabi/BP_Character_Player.LBUIPressEOff` _asbp_character_player))

(event `GetEnableEnergy`
  ;[1 1 1] Put Fuse in Fusebox
  (bind _outactors (`GameplayStatics.GetAllActorsOfClass` "/Game/Blueprints/BP_Reactor.BP_Reactor_C"))
  (add `/Game/Blueprints/BP_Reactor.EnableEnergy` (`KismetArrayLibrary.Array_Get` _outactors) (delegate `EnableEnergy`)))

(event `self.Box.OnComponentEndOverlap`
  (params (OverlappedComponent :type "PrimitiveComponent Object Reference") (OtherActor :type "Actor Object Reference") (OtherComp :type "PrimitiveComponent Object Reference") (OtherBodyIndex :type Integer))
  ;[1 1 1] Put Fuse in Fusebox
  ;;[1 1 1] Enable/Disable UI
  (goto _label))

(event `EnableEnergy`
  (bind _defaultintensity (`self.DefaultIntensity`))
  ;[1 1 1] Put Fuse in Fusebox
  (bind (_direction _newtrack_1) (`Timeline|Timeline_2` :!via `PlayFromStart`)
    (:`Update`
      (`LightComponent.SetIntensity` (`self.SpotLight`) (`KismetMathLibrary.Lerp` (* _defaultintensity 0.1) _defaultintensity _newtrack_1)))))

(fn `UserConstructionScript`)