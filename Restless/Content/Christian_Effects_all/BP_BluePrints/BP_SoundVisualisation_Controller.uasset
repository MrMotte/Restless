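; Controller that drives a sound visualiser, scaling the height of BP_SoundVisualisation_Bar actors in the level to an audio frequency spectrum.
; On BeginPlay it gathers the bars, insertion-sorts them by X position and starts the audio component on its Sound.
; Each tick it samples the spectrum of RadioCall2 slightly ahead of game time and sets each bar's Z scale from its band's clamped, cubed value.
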(event `self.ReceiveBeginPlay`
  (bind _audio (`self.Audio`))
  (bind _outactors (`GameplayStatics.GetAllActorsOfClass` "/Game/Christian_Effects_all/BP_BluePrints/BP_SoundVisualisation_Bar.BP_SoundVisualisation_Bar_C"))
  (for _array_element _outactors
    (for (_array_element_2 _array_index) _
      (if (not (> (.x (`self.K2_GetActorLocation` _array_element_2)) (.x (`self.K2_GetActorLocation` _array_element))))
        (break)))
    (`KismetArrayLibrary.Array_Insert` (`self.Bar`) null _array_index)
    (`AudioComponent.SetSound` _audio (`self.Sound`))
    (`AudioComponent.Play` _audio 0.0)))

(event `self.ReceiveTick`
  (params (DeltaSeconds :type "Float (single-precision)"))
  (bind _outspectrum (`SoundVisualizationStatics.CalculateFrequencySpectrum` "/Game/Sounds/Voice/RadioCall2.RadioCall2" 0 (+ (`KismetSystemLibrary.GetGameTimeInSeconds`) 0.08) 0.19 3))
  (set `self.Frequencies` _outspectrum)
  (for (_array_element _array_index) (`self.Bar`)
    (bind _returnvalue (`KismetMathLibrary.FClamp` (/ (`KismetArrayLibrary.Array_Get` (`self.Frequencies`) _array_index) 3.0) 0.0 5000.0))
    (`self.SetActorScale3D` _array_element (`KismetMathLibrary.MakeVector` 1.0 1.0 (+ (* _returnvalue _returnvalue _returnvalue) 0.1)))))

(fn `UserConstructionScript`)